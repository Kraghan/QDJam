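; BP_BaseBall is a base ball actor that travels along a trajectory spline and destroys itself on reaching a goal or player.
; Tick accumulates lifetime and, using Lifetime divided by Speed as spline time, moves the ball with swept location updates.
; Past the spline's end, it keeps moving by the last per-frame offset, continuing straight.
; OnEnterGoal and OnEnterPlayer print a debug message before destroying the ball.
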(event `self.ReceiveTick`
  (params (DeltaSeconds :type "Float (single-precision)"))
  (bind _output_get (set `self.Lifetime` (+ DeltaSeconds (`self.Lifetime`))))
  (bind _returnvalue (/ _output_get (`self.Speed`)))
  (if (>= _returnvalue 1.0)
    (`self.K2_SetActorLocation` (+ (`self.LastMoveDir`) (`self.K2_GetActorLocation`)) true)
    (else
      (bind _output_get_2 (set `self.PreviousPos` (`self.K2_GetActorLocation`)))
      (bind _returnvalue_2 (`SplineComponent.GetLocationAtTime` (`/Game/Blueprints/Game/BP_ShootTrajectory.Spline` (`self.Trajectory`)) _returnvalue "World" false))
      (`self.K2_SetActorLocation` _returnvalue_2 true)
      (set `self.LastMoveDir` (- _returnvalue_2 _output_get_2)))))

(fn `OnEnterGoal`
  (`KismetSystemLibrary.PrintString` "Ball reached goal")
  (`self.K2_DestroyActor`))

(fn `OnEnterPlayer`
  (`KismetSystemLibrary.PrintString` "Ball reached player !")
  (`self.K2_DestroyActor`))

(fn `UserConstructionScript`)