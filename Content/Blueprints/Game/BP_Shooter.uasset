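; BP_Shooter is an actor that launches balls on a timed schedule defined by its ShootSequence array.
; Each Tick, HandleSequence advances an elapsed-time counter and checks every entry's StartTime against the interval since the previous frame.
; Entries falling in that window spawn their BallObject class at the ShootTrajectory's origin, passing in the trajectory and speed, so each fires once without needing a fired flag.
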(event `self.ReceiveTick`
  (params (DeltaSeconds :type "Float (single-precision)"))
  (`self.HandleSequence` DeltaSeconds))

(fn `HandleSequence`
  (params (DeltaTime :type "Float (double-precision)"))
  (locals (PreviousTime :type "Float (double-precision)"))
  (bind _timeelapsed (`self.TimeElapsed`))
  (bind _output_get (set `local.PreviousTime` _timeelapsed))
  (bind _output_get_2 (set `self.TimeElapsed` (+ _timeelapsed DeltaTime)))
  (for _array_element (`self.ShootSequence`)
    (if (and (<= (`.StartTime_13_60EDDC764844F338E43BA488A53537BA` (break `/Game/Blueprints/Game/ST_ShootOrdonancer` _array_element)) _output_get_2) (> (`.StartTime_13_60EDDC764844F338E43BA488A53537BA` (break `/Game/Blueprints/Game/ST_ShootOrdonancer` _array_element)) _output_get))
      (`|SpawnActorFromClass` (`.BallObject_14_78D77EC4436E29CD937D38ACC96C41CB` (break `/Game/Blueprints/Game/ST_ShootOrdonancer` _array_element)) (`KismetMathLibrary.MakeTransform` (`/Game/Blueprints/Game/BP_ShootTrajectory.GetShootOrigin` (break `/Game/Blueprints/Game/ST_ShootOrdonancer` _array_element))) "Undefined" "MultiplyWithRoot" null (break `/Game/Blueprints/Game/ST_ShootOrdonancer` _array_element) (`.Speed_10_51B600904A89E434614E06822152F99E` (break `/Game/Blueprints/Game/ST_ShootOrdonancer` _array_element)) null))))

(fn `UserConstructionScript`)