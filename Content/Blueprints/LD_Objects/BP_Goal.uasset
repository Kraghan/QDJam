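; BP_Goal is a goal actor that loses health whenever a ball enters it.
; On BeginPlay it creates the WBP_HeartHUD widget with a reference to itself, adds it to the viewport and resets health to maximum.
; A BP_BaseBall overlapping its box is notified via OnEnterGoal, then the goal drops one health point and calls the OnTakeDamage dispatcher.
; It contains no handling for health reaching zero.
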(event `self.ReceiveBeginPlay`
  (bind _returnvalue (`|CreateWidget` "/Game/UI/WBP_HeartHUD.WBP_HeartHUD_C" null self))
  (`UserWidget.AddToViewport` _returnvalue 0)
  (set `self.CurrentHealth` (`self.MaxHealth`)))

(event `self.Box.OnComponentBeginOverlap`
  (params (OverlappedComponent :type "PrimitiveComponent Object Reference") (OtherActor :type "Actor Object Reference") (OtherComp :type "PrimitiveComponent Object Reference") (OtherBodyIndex :type Integer) (bFromSweep :type Boolean) (SweepResult :type "HitResult Structure (by ref)"))
  (bind _asbp_base_ball (cast `/Game/Blueprints/Game/BP_BaseBall` OtherActor))
  (`/Game/Blueprints/Game/BP_BaseBall.OnEnterGoal` _asbp_base_ball)
  (`/Engine/EditorBlueprintResources/StandardMacros.DecrementInt` (`self.CurrentHealth`)
    (:`  `
      (`self.OnTakeDamage`))))

(fn `UserConstructionScript`)